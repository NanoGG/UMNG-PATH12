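; Stair trigger actor (Escalera) that teleports the player to another floor behind a fade.
; On any overlap it sets TriggerEscalera on the Personaje as a re-entry guard, without checking which actor overlapped.
; It shows the Fade widget, moves the player to NuevaPos with control rotation NuevaRot, then clears the guard.
; A PisoNuevo widget then briefly displays the new floor name from PisoNombre.
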(event EventBeginPlay
  (bind _returnvalue (UserInterface|CreateWidget "/Game/Widgets_recorrido/Recorrido/Fade.Fade_C"))
  (Variables|Default|Setfade_wid _returnvalue))

(event Collision|EventActorBeginOverlap
  (params (OtherActor :type Actor%20Object%20Reference))
  (bind _fade_wid (Variables|Default|Getfade_wid))
  (bind _returnvalue (Actor|GetActorOfClass "/Game/Blueprints/personaje.personaje_C"))
  (if (not (Variables|/Game/Blueprints/personaje.personaje_C|GetTriggerEscalera _returnvalue))
    (Variables|/Game/Blueprints/personaje.personaje_C|SetTriggerEscalera _returnvalue true)
    (if (not (UserInterface|Viewport|IsinViewport (Variables|Default|Getfade_wid)))
      ;[1 1 1] Fade out
      (UserInterface|Viewport|AddtoViewport _fade_wid 0)
      (Utilities|FlowControl|Delay 1.0)
      (Widget|RemovefromParent _fade_wid)
      ;[1 1 1] Reubicar posicion y rotación del jugador
      (bind _returnvalue_2 (Actor|GetActorOfClass "/Game/Blueprints/personaje.personaje_C"))
      (Transformation|SetActorLocation _returnvalue_2 (Variables|Default|GetNueva_pos) false true)
      (Pawn|SetControlRotation (Game|GetPlayerController 0) (Variables|Default|GetNueva_rot))
      (bind _returnvalue_3 (Actor|GetActorOfClass "/Game/Blueprints/personaje.personaje_C"))
      (Variables|/Game/Blueprints/personaje.personaje_C|SetTriggerEscalera _returnvalue_3 false)
      ;[1 1 1] Mostrar en que piso esta ahora
      (bind _returnvalue_4 (UserInterface|CreateWidget "/Game/Widgets_recorrido/Recorrido/PisoNuevo.PisoNuevo_C"))
      (Rendering|Components|TextRender|SetText (Variables|/Game/Widgets_recorrido/Recorrido/PisoNuevo.PisoNuevo_C|GetPiso_texto _returnvalue_4) (Utilities|Text|ToText(String) (Variables|Default|GetPiso_nombre)))
      (UserInterface|Viewport|AddtoViewport _returnvalue_4 0)
      (Utilities|FlowControl|Delay 1.0)
      (Widget|RemovefromParent _returnvalue_4))))

(event EventTick
  (params (DeltaSeconds :type Float%20%28single-precision%29)))

(fn ConstructionScript)