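; Global_vars is a Blueprint that builds a shared list of place names for the character's current site (SedeActual).
; LlenarListaLugares clears ListaLugares, then finds the Personaje actor with GetActorOfClass to read its SedeActual.
; Nested loops walk that site's Bloques and their Lugares, appending each NombreLugar to the flat list.
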(fn LlenarListaLugares
  (Utilities|Array|Clear (Variables|Default|GetLista_lugares))
  (bind _returnvalue (Actor|GetActorOfClass "/Game/Blueprints/personaje.personaje_C"))
  (for _array_element (Variables|/Game/Blueprints/Sede.Sede_C|GetBloques (Variables|/Game/Blueprints/personaje.personaje_C|GetSede_actual _returnvalue))
    (for _array_element_2 (Variables|/Game/Blueprints/Bloque.Bloque_C|GetLugares _array_element)
      (Utilities|Array|Add (Variables|Default|GetLista_lugares) (Variables|/Game/Blueprints/Lugar.Lugar_C|GetNombre_lugar _array_element_2)))))