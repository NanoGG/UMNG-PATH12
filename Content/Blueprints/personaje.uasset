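; Player character for a campus navigation app, with manual movement, auto-follow, fast travel and GPS positioning at Calle100 or Cajica.
; A fast looping timer reads Global_vars to move toward Destino, redraws the navmesh route as short-lived debug lines, and shows an arrival widget when close.
; A one-second timer converts latitude/longitude offsets from the campus origin into actor location.
; VerficarDestino resolves the destination name among the current campus's blocks.
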(event Custom|MoveActor
  ;[1 1 1] Ajuste de posición del GPS
  (if (and (Variables|Default|GetGPS_Activacion) (or (Variables|Default|GetPlayInCalle100) (Variables|Default|GetPlayInCajica)))
    (if (Variables|Default|GetPlayInCalle100)
      (if (Variables|Default|GetIsInCalle100)
        (Class|LocationServices|StartLocationServices)
        (bind _returnvalue (Class|LocationServices|GetLastKnownLocation))
        (bind _output_get (Variables|Default|SetCoorD (Math|Vector|MakeVector (- (.latitude _returnvalue) (Variables|Default|GetLatCalle100)) (- (.longitude _returnvalue) (Variables|Default|GetLongCalle100)) 0.0)))
        (Transformation|SetActorLocation (Game|GetPlayerCharacter 0) (+ (* (* _output_get 111.120003) 100000) "0, 0,112.000000") false false))
      (elif (Variables|Default|GetIsInCajica)
        (Class|LocationServices|StartLocationServices)
        (bind _returnvalue_2 (Class|LocationServices|GetLastKnownLocation))
        (bind _output_get_2 (Variables|Default|SetCoorD (Math|Vector|MakeVector (- (.latitude _returnvalue_2) (Variables|Default|GetLatCajica)) (- (.longitude _returnvalue_2) (Variables|Default|GetLongCajica)) 0.0)))
        (Transformation|SetActorLocation (Game|GetPlayerCharacter 0) (+ (* (* _output_get_2 111.120003) 100000) "0, 0,112.000000") false false)))))

(event Custom|Ruta
  (bind _self self)
  ;[1 1 1] Generacion de ruta y movimiento automatico
  (Utilities|FlowControl|Sequence
    (:then_0
      (CallFunction|SeguimientoAuto)
      (CallFunction|ViajarRapido))
    (:then_1
      (bind _asglobal_vars (Utilities|Casting|CastToGlobal_vars (Game|GetGameInstance)))
      (Variables|Default|SetGlobal%20Vars%20ref _asglobal_vars)
      (if (Variables|/Game/Blueprints/Global_vars.Global_vars_C|GetGenerar_ruta _asglobal_vars)
        (bind _esta_cerca (CallFunction|VerificarCercania))
        (if _esta_cerca
          (if (Math|Boolean|Equal(Boolean) (Variables|Default|GetEsta_en_interior _self) (Variables|/Game/Blueprints/Lugar.Lugar_C|GetEsta_en_interior (Variables|Default|GetDestino _self)))
            (Utilities|FlowControl|Sequence
              (:then_0
                (if (Variables|/Game/Blueprints/Global_vars.Global_vars_C|GetSeguir_auto (Variables|Default|GetGlobal%20Vars%20ref))
                  (Variables|/Game/Blueprints/Global_vars.Global_vars_C|SetSeguir_auto (Variables|Default|GetGlobal%20Vars%20ref) false)))
              (:then_1
                (Widget|SetVisibility (Variables|Default|GetLlegaste) "Visible")
                (Variables|/Game/Blueprints/Global_vars.Global_vars_C|SetLlego_a_destino (Variables|Default|GetGlobal%20Vars%20ref) true)
                (Variables|/Game/Blueprints/Global_vars.Global_vars_C|SetGenerar_ruta (Variables|Default|GetGlobal%20Vars%20ref) false)
                (Variables|/Game/Blueprints/Global_vars.Global_vars_C|SetHay_destino (Variables|Default|GetGlobal%20Vars%20ref) false)
                (Utilities|FlowControl|Delay 1.5)
                (Widget|SetVisibility (Variables|Default|GetLlegaste) "Hidden"))
              (:then_2
                (Widget|RemovefromParent (Variables|Default|GetAuto))
                (Widget|RemovefromParent (Variables|Default|GetViaje%20Rapido)))
              (:then_3
                (bind _foundwidgets (Widget|GetAllWidgetsOfClass "/Game/Menu/Widgets/Barra_busqueda.Barra_busqueda_C" true))
                (Class|EditableTextBox|SetHintText (Variables|/Game/Menu/Widgets/Barra_busqueda.Barra_busqueda_C|GetBarraBusqueda (Utilities|Array|Get(acopy) _foundwidgets)) "Buscar destino"))))
          (else
            (CallFunction|GenerarRuta (Transformation|GetActorLocation (Variables|Default|GetDestino self)) (+ 0.0 0.01))))))))

(event EventBeginPlay
  ;[1 1 1] Permisos de acceso al GPS
  (Utilities|FlowControl|Sequence
    (:then_0
      (bind _returnvalue (UserInterface|CreateWidget "/Game/Widgets_recorrido/Recorrido/DestinoAlcanzado.DestinoAlcanzado_C"))
      (bind _output_get (Variables|Default|SetLlegaste _returnvalue))
      (UserInterface|Viewport|AddtoViewport _output_get 0)
      (Widget|SetVisibility _output_get "Hidden")
      (Utilities|FlowControl|Sequence
        (:then_0
          (bind _returnvalue_2 (UserInterface|CreateWidget "/Game/Widgets_recorrido/Recorrido/Automatico.Automatico_C"))
          (Variables|Default|SetAuto _returnvalue_2)
          (bind _returnvalue_3 (UserInterface|CreateWidget "/Game/Widgets_recorrido/Recorrido/ViajeRapido.ViajeRapido_C"))
          (Variables|Default|SetViaje%20Rapido _returnvalue_3))
        (:then_1
          (bind _asglobal_vars (Utilities|Casting|CastToGlobal_vars (Game|GetGameInstance)))
          (if (Variables|/Game/Blueprints/Global_vars.Global_vars_C|GetGenerar_ruta _asglobal_vars)
            (UserInterface|Viewport|AddtoViewport (Variables|Default|GetAuto self) 0)
            (UserInterface|Viewport|AddtoViewport (Variables|Default|GetViaje%20Rapido self) 0)))))
    (:then_1
      (bind _returnvalue_4 (Class|LocationServices|InitLocationServices "LA_TenMeters" 0.0 0.0))
      (bind _output_get_2 (Variables|Default|SetInit%20location%20services _returnvalue_4))
      (if _output_get_2
        _))
    (:then_2
      (Utilities|Time|SetTimerbyEvent (delegate Custom|MoveActor) 1.0 true))
    (:then_3
      ;[1 1 1] Generacion de ruta y movimiento automatico
      (Utilities|Time|SetTimerbyEvent (delegate Custom|Ruta) (+ 0.0 0.01) true))))

(event Input|AxisEvents|InputAxisMoveForward
  (params (AxisValue :type Float%20%28single-precision%29))
  ;[1 1 1] Movimiento
  (Pawn|Input|AddMovementInput (Math|Vector|GetForwardVector (Math|Rotator|MakeRotator 0.0 0.0 (.Yaw (Math|Rotator|BreakRotator (Pawn|GetControlRotation :!class /Script/Engine.Pawn))))) AxisValue false))

(event Input|AxisEvents|InputAxisMoveRight
  (params (AxisValue :type Float%20%28single-precision%29))
  ;[1 1 1] Movimiento
  (Pawn|Input|AddMovementInput (Math|Vector|GetRightVector (Math|Rotator|MakeRotator 0.0 0.0 (.Yaw (Math|Rotator|BreakRotator (Pawn|GetControlRotation :!class /Script/Engine.Pawn))))) AxisValue false))

(event Input|AxisEvents|InputAxisTurnRate
  (params (AxisValue :type Float%20%28single-precision%29))
  ;[1 1 1] Movimiento
  (Pawn|Input|AddControllerYawInput (* AxisValue 45.0 (Utilities|Time|GetWorldDeltaSeconds))))

(event Input|AxisEvents|InputAxisLookUpRate
  (params (AxisValue :type Float%20%28single-precision%29))
  ;[1 1 1] Movimiento
  (Pawn|Input|AddControllerPitchInput (* AxisValue 45.0 (Utilities|Time|GetWorldDeltaSeconds))))

(fn ConstructionScript)

(fn GenerarRuta
  (params (Ubicacion_destino :type Vector) (Tick :type Float%20%28single-precision%29))
  (bind _returnvalue (+ Tick 0.005))
  (bind _self self)
  (if (== (Variables|Default|GetEscala self) 1)
    (LocalVariables|Setmultiplo 275.0)
    (bind _returnvalue_2 (Class|NavigationSystemV1|FindPathtoLocationSynchronously (+ (* (Math|Vector|GetForwardVector (Variables|Collision|GetCapsuleComponent _self)) (LocalVariables|Getmultiplo)) (Transformation|GetActorLocation _self)) Ubicacion_destino (Variables|Default|GetNavmesh_actual self) 0))
    (Utilities|FlowControl|Sequence
      (:then_1
        (for (_array_element _array_index) (Variables|/Script/NavigationSystem.NavigationPath|GetPathPoints _returnvalue_2)
          (switch int _array_index
            (:Default
              (Rendering|Debug|DrawDebugLine (+ (Utilities|Array|Get(acopy) (Variables|/Script/NavigationSystem.NavigationPath|GetPathPoints _returnvalue_2) (- _array_index 1)) "0, 0,80.000000") (+ _array_element "0, 0,80.000000") "(R=0.250158,G=0.001518,B=0.002428,A=1.000000)" _returnvalue 3e+01))))))
    (elif (== (Variables|Default|GetEscala) 2)
      (LocalVariables|Setmultiplo 215.0)
      (bind _returnvalue_3 (Class|NavigationSystemV1|FindPathtoLocationSynchronously (+ (* (Math|Vector|GetForwardVector (Variables|Collision|GetCapsuleComponent _self)) (LocalVariables|Getmultiplo)) (Transformation|GetActorLocation _self)) Ubicacion_destino (Variables|Default|GetNavmesh_actual self) 0))
      (Utilities|FlowControl|Sequence
        (:then_1
          (for (_array_element_2 _array_index_2) (Variables|/Script/NavigationSystem.NavigationPath|GetPathPoints _returnvalue_3)
            (switch int _array_index_2
              (:Default
                (Rendering|Debug|DrawDebugLine (+ (Utilities|Array|Get(acopy) (Variables|/Script/NavigationSystem.NavigationPath|GetPathPoints _returnvalue_3) (- _array_index_2 1)) "0, 0,2.000000") (+ _array_element_2 "0, 0,2.000000") "(R=0.250158,G=0.001518,B=0.002428,A=1.000000)" _returnvalue 2e+01)))))))))

(fn SeguimientoAuto
  (bind _self self)
  (bind _returnvalue (Pawn|GetController _self))
  (bind _asglobal_vars (Utilities|Casting|CastToGlobal_vars (Game|GetGameInstance)))
  (if (Variables|/Game/Blueprints/Global_vars.Global_vars_C|GetSeguir_auto _asglobal_vars)
    (AI|Navigation|SimpleMovetoActor _returnvalue (Variables|Default|GetDestino _self))
    (if (Variables|/Game/Blueprints/Global_vars.Global_vars_C|GetLlego_a_destino _asglobal_vars)
      (Variables|/Game/Blueprints/Global_vars.Global_vars_C|SetSeguir_auto _asglobal_vars false))
    (else
      (AI|Navigation|StopMovement _returnvalue))))

(fn VerificarCercania
  (bind _self self)
  (bind _self_2 self)
  (bind _returnvalue (Transformation|GetActorLocation _self_2))
  (bind _destino (Variables|Default|GetDestino _self))
  (bind _capsulecomponent (Variables|Collision|GetCapsuleComponent _self_2))
  (bind _returnvalue_2 (Math|Vector|GetForwardVector _capsulecomponent))
  (bind _returnvalue_3 (Transformation|GetActorLocation _destino))
  (bind _returnvalue_4 (* _returnvalue_2 2.4e+02))
  (bind _returnvalue_5 (+ _returnvalue_4 _returnvalue))
  (bind _returnvalue_6 (- _returnvalue_3 _returnvalue_5))
  (bind _returnvalue_7 (Math|Vector|VectorLength _returnvalue_6))
  (if (Variables|Default|GetEsta_en_interior self)
    (LocalVariables|SetCerca (<= _returnvalue_7 3e+02))
    (else
      (LocalVariables|SetCerca (<= _returnvalue_7 3.5e+02))))
  (return (LocalVariables|GetCerca)))

(fn VerficarDestino
  (bind _asglobal_vars (Utilities|Casting|CastToGlobal_vars (Game|GetGameInstance)))
  (if (Variables|/Game/Blueprints/Global_vars.Global_vars_C|GetGenerar_ruta _asglobal_vars)
    (if (not (Utilities|Enum|Equal(Enum) (Utilities|GetObjectName (Variables|Default|GetDestino self)) (Variables|/Game/Blueprints/Global_vars.Global_vars_C|GetDestino_nom _asglobal_vars)))
      (for _array_element (Variables|/Game/Blueprints/Sede.Sede_C|GetBloques (Variables|personaje_C|GetSede_actual self))
        (for _array_element_2 (Variables|/Game/Blueprints/Bloque.Bloque_C|GetLugares _array_element)
          (if (Utilities|Enum|Equal(Enum) (Utilities|GetObjectName _array_element_2) (Variables|/Game/Blueprints/Global_vars.Global_vars_C|GetDestino_nom _asglobal_vars))
            (Variables|Default|SetDestino self _array_element_2)
            (LocalVariables|SetEncontrado true))))
      (if (not (LocalVariables|GetEncontrado))
        (Variables|/Game/Blueprints/Global_vars.Global_vars_C|SetGenerar_ruta _asglobal_vars false)
        (Variables|/Game/Blueprints/Global_vars.Global_vars_C|SetHay_destino _asglobal_vars false)
        (Variables|/Game/Blueprints/Global_vars.Global_vars_C|SetLlego_a_destino _asglobal_vars true)
        (Variables|/Game/Blueprints/Global_vars.Global_vars_C|SetDestino_nom _asglobal_vars "")
        (Development|PrintString "DESTINO NO ENCONTRADO" true true "(R=1.000000,G=0.308127,B=0.212375,A=1.000000)")))))

(fn ViajarRapido
  (bind _self self)
  (bind _asglobal_vars (Utilities|Casting|CastToGlobal_vars (Game|GetGameInstance)))
  (if (Variables|/Game/Blueprints/Global_vars.Global_vars_C|GetUsa_viaje_rapido _asglobal_vars)
    (Transformation|SetActorLocation (Transformation|GetActorLocation (Variables|Default|GetDestino self)) false true)
    (if (Math|Boolean|Equal(Boolean) (Variables|Default|GetEsta_en_interior _self) (Variables|/Game/Blueprints/Lugar.Lugar_C|GetEsta_en_interior (Variables|Default|GetDestino _self)))
      (Variables|/Game/Blueprints/Global_vars.Global_vars_C|SetUsa_viaje_rapido _asglobal_vars false))))